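; BP_Jellyfish is an actor that animates a jellyfish bobbing along the vertical axis around its placed location.
; On BeginPlay it stores its start location, waits a random few seconds, then plays the Swim timeline, whose SpeedCurve sets the Z offset from that start.
; Each finished play triggers another random pause and a replay from the beginning, so the motion loops at irregular intervals.
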(event EventBeginPlay
  (Variables|Default|SetStart (Transformation|GetActorLocation))
  (Utilities|FlowControl|Delay (Math|Random|RandomFloatinRange 1.0 4.0))
  (bind _speedcurve (Timeline|swim Play)
    (:Update
      (Transformation|SetActorLocation (+ (Math|Vector|MakeVector 0.0 0.0 _speedcurve) (Variables|Default|GetStart)) false false))
    (:Finished
      (Utilities|FlowControl|Delay (Math|Random|RandomFloatinRange 1.0 4.0))
      (Timeline|swim PlayFromStart))))

(event Collision|EventActorBeginOverlap
  (params (OtherActor :type Actor%20Object%20Reference)))

(event EventTick
  (params (DeltaSeconds :type Float%20%28single-precision%29)))

(fn ConstructionScript)