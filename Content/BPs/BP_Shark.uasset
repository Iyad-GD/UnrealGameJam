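; BP_Shark is a shark actor that swims continuously along a spline path placed in the level.
; BeginPlay caches the spline length, then each Tick advances a distance by speed and delta time, wrapping with modulo to loop.
; The skeletal mesh is moved to that world-space point and rotated to face the spline direction, with a fixed yaw offset to correct the mesh orientation.
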(event EventBeginPlay
  (Variables|Default|SetSplineLength (Spline|GetSplineLength (Variables|Default|GetSpline))))

(event EventTick
  (params (DeltaSeconds :type Float%20%28single-precision%29))
  (bind _output_get (Variables|Default|SetDistance (Math|Float|%(Float) (+ (* DeltaSeconds (Variables|Default|GetSpeed)) (Variables|Default|GetDistance)) (Variables|Default|GetSplineLength))))
  (Transformation|SetWorldLocation (Variables|Default|GetSkeletalMesh) (Spline|GetLocationatDistanceAlongSpline (Variables|Default|GetSpline) _output_get "World") false false)
  (Transformation|SetWorldRotation (Variables|Default|GetSkeletalMesh) (Math|Rotator|CombineRotators (Math|Rotator|MakeRotfromX (Spline|GetDirectionatDistanceAlongSpline (Variables|Default|GetSpline) _output_get "World")) "0.000000,-90.000000,0.000000") false false))

(fn ConstructionScript)